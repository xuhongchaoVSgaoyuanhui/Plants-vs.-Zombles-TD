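; BP_tombstone is a tombstone actor whose components represent menu entries: Adventure, Challenge, Survival, Book, Option, Help and Quit.
; Two custom events, 字符放大 (enlarge) and 字符缩小 (shrink), switch on a Text argument and set the matching component's world scale to a fixed larger or smaller size.
; It has no active BeginPlay, overlap or Tick logic, so scaling changes only when these events are called.
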(event `字符放大`
  (params (text :type "/Game/UI/M_UItext Enum" :default "NewEnumerator0"))
  (switch `/Game/UI/M_UItext` text
    (:`NewEnumerator0`
      (`SceneComponent.SetWorldScale3D` (`self.Adventure mode`) (0.8 0.8 0.8)))
    (:`NewEnumerator1`
      (`SceneComponent.SetWorldScale3D` (`self.Challenge mode`) (0.8 0.8 0.8)))
    (:`NewEnumerator2`
      (`SceneComponent.SetWorldScale3D` (`self.Survival mode`) (0.8 0.8 0.8)))
    (:`NewEnumerator6`
      (`SceneComponent.SetWorldScale3D` (`self.book`) (0.35 0.5 0.65)))
    (:`NewEnumerator3`
      (`SceneComponent.SetWorldScale3D` (`self.option`) (1.0 0.55 0.55)))
    (:`NewEnumerator4`
      (`SceneComponent.SetWorldScale3D` (`self.help`) (1.0 0.55 0.55)))
    (:`NewEnumerator5`
      (`SceneComponent.SetWorldScale3D` (`self.quit`) (1.0 0.55 0.8)))))

(event `字符缩小`
  (params (text :type "/Game/UI/M_UItext Enum" :default "NewEnumerator0"))
  (switch `/Game/UI/M_UItext` text
    (:`NewEnumerator0`
      (`SceneComponent.SetWorldScale3D` (`self.Adventure mode`) (0.7 0.7 0.7)))
    (:`NewEnumerator1`
      (`SceneComponent.SetWorldScale3D` (`self.Challenge mode`) (0.7 0.7 0.7)))
    (:`NewEnumerator2`
      (`SceneComponent.SetWorldScale3D` (`self.Survival mode`) (0.7 0.7 0.7)))
    (:`NewEnumerator6`
      (`SceneComponent.SetWorldScale3D` (`self.book`) (0.35 0.2 0.35)))
    (:`NewEnumerator3`
      (`SceneComponent.SetWorldScale3D` (`self.option`) (1.0 0.25 0.25)))
    (:`NewEnumerator4`
      (`SceneComponent.SetWorldScale3D` (`self.help`) (1.0 0.25 0.25)))
    (:`NewEnumerator5`
      (`SceneComponent.SetWorldScale3D` (`self.quit`) (1.0 0.25 0.25)))))

(fn `UserConstructionScript`)